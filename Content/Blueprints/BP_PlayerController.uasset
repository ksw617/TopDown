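; Player controller for click-to-move control of the pawn with the mouse, using Enhanced Input and a mouse mapping context added on BeginPlay.
; Pressing stops current movement; while held, a visibility trace under the cursor caches the destination and steers the pawn straight toward it.
; A short click, released or canceled, instead calls SimpleMoveToLocation to the cached point and spawns a cursor effect there.
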(event `self.ReceiveBeginPlay`
  (bind _returnvalue (subsystem `EnhancedInputLocalPlayerSubsystem`))
  (`/Engine/EditorBlueprintResources/StandardMacros.IsValid` _returnvalue
    (:`Is Valid`
      (`EnhancedInputSubsystemInterface.AddMappingContext` _returnvalue "/Game/Input/IMC_Mouse.IMC_Mouse" 0 (struct)))))

(event `EnhancedInput|/Game/Input/IA_MouseClick`
  (params (ActionValue :type Boolean) (ElapsedSeconds :type "Float (double-precision)") (TriggeredSeconds :type "Float (double-precision)") (InputAction :type "InputAction Object Reference" :default "/Game/Input/IA_MouseClick.IA_MouseClick"))
  (bind (_bblockinghit _location) (`self.GetLocationUnderCursor`))
  (bind _cacheddestination (`self.CachedDestination`))
  (:`Triggered`
    (if _bblockinghit
      (bind _output_get (set `self.CachedDestination` _location))
      (`self.Follow` _output_get)))
  (:`Started`
    (`self.StopMovement`))
  (:`Canceled`
    (if (< ElapsedSeconds 0.5) :!label _label
      (`AIBlueprintHelperLibrary.SimpleMoveToLocation` self _cacheddestination)
      (`NiagaraFunctionLibrary.SpawnSystemAtLocation` "/Game/Cursor/FX_Cursor.FX_Cursor" _cacheddestination)))
  (:`Completed`
    (goto _label)))

(fn `Follow`
  (params (Location :type "Vector Structure"))
  (bind _returnvalue (`self.K2_GetPawn`))
  (`Pawn.AddMovementInput` _returnvalue (`KismetMathLibrary.GetDirectionUnitVector` (`self.K2_GetActorLocation` _returnvalue) Location) 1.0 false))

(fn `GetLocationUnderCursor`
  (returns (bBlockingHit :type Boolean) (Location :type "Vector Structure"))
  (bind (_bblockinghit _binitialoverlap _time _distance _location) (`GameplayStatics.BreakHitResult` (`self.GetHitResultUnderCursorByChannel` "TraceTypeQuery1")))
  (return _bblockinghit _location))

(fn `UserConstructionScript`)